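; PN_SkilledNinja is a prop-ninja actor that follows the player's camera aim until its skill is fired.
; Each Tick calls an event dispatcher, bound on BeginPlay if PNSPlayerVessel is valid, to run UpdateLocation.
; UpdateLocation line-traces ahead for blocker objects, placing the actor just above a hit or at maximum range.
; FireSkill only prints a message, then triggers Deconstruct to detach and destroy the actor.
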(event `self.ReceiveBeginPlay`
  (if (`KismetSystemLibrary.IsValid` (`self.PN_S_PlayerVessel`))
    (add `self.UpdateLocEventDisp` (delegate `UpdateLocEvent`))))

(event `self.ReceiveTick`
  (params (DeltaSeconds :type "Float (single-precision)"))
  (`self.UpdateLocEventDisp`))

(event `UpdateLocEvent`
  (`self.UpdateLocation`))

(event `Deconstruct`
  (if (`self.Decon`)
    (`self.K2_DetachFromActor` "KeepRelative")
    (`self.K2_DestroyActor`)))

(fn `FireSkill`
  (`KismetSystemLibrary.PrintText` "Firing Ninja.")
  (set `self.Decon` true)
  (`self.Deconstruct`)
  (return))

(fn `UpdateLocation`
  (bind _pn_s_playervessel (`self.PN_S_PlayerVessel`))
  (bind _returnvalue (`self.K2_GetActorLocation` _pn_s_playervessel))
  (bind _returnvalue_2 (+ _returnvalue (* (`SceneComponent.GetForwardVector` (`/Game/Blueprints/Archetypes/PlayerVessel.PlayerCam` _pn_s_playervessel)) 600.0)))
  (bind (_outhit _returnvalue_3) (`KismetSystemLibrary.LineTraceSingleForObjects` _returnvalue _returnvalue_2 (`self.TargetBlockerObjectTypes`)))
  (if _returnvalue_3
    (`self.K2_SetActorLocation` (+ (`.Location` (`GameplayStatics.BreakHitResult` _outhit)) (0.0 0.0 10.0)))
    (return)
    (else
      (`self.K2_SetActorLocation` _returnvalue_2)
      (return))))

(fn `UserConstructionScript`)