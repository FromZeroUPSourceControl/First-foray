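; Sword Rain skill actor for PropNinjas that rains RainySword actors down over a magic circle.
; Tick counter-rotates the circle and sparkles, and FireSkill unbinds the location-update dispatcher before starting the volley.
; RepFire re-calls itself after short delays, spawning swords at random overhead offsets until SwordCount runs out, then calls Deconstruct.
; FireSwords, a fixed four-sword pattern, is not called within this Blueprint.
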(event `self.ReceiveTick`
  (params (DeltaSeconds :type "Float (single-precision)"))
  (`parent.ReceiveTick` DeltaSeconds)
  (`SceneComponent.K2_AddRelativeRotation` (`self.MagicCircle`) (struct :`Yaw` 1.0) false false)
  (`SceneComponent.K2_AddRelativeRotation` (`self.MagicSparkles`) (struct :`Yaw` -0.3) false false))

(event `RepFire`
  (bind _swordcount (`self.SwordCount`))
  (if (> _swordcount 0) :!label _label
    (`/Engine/EditorBlueprintResources/StandardMacros.DecrementInt` _swordcount
      (:`  `
        (`KismetSystemLibrary.Delay` 0.1)
        (`self.FireSword`)
        (`self.RepFire`)))
    (else
      (set `self.Decon` true)
      (`self.Deconstruct`))))

(event `self.FireSkill`
  (clear `self.UpdateLocEventDisp`)
  (goto _label))

(fn `FireSword`
  (locals (BeanCounter :type "Vector Structure" :default (0.0 0.0 800.0)))
  (set `local.BeanCounter` (`KismetMathLibrary.MakeVector` (* (- (`KismetMathLibrary.RandomFloat`) 0.5) 400.0) (* (- (`KismetMathLibrary.RandomFloat`) 0.5) 400.0) (+ (* (`KismetMathLibrary.RandomFloat`) 100.0) 800.0)))
  (`|SpawnActorFromClass` "/Game/Blueprints/Damage/RainySword.RainySword_C" (`KismetMathLibrary.MakeTransform` (+ (`SceneComponent.K2_GetComponentLocation` (`self.DefaultSceneRoot`)) (`local.BeanCounter`)) (`KismetMathLibrary.MakeRotator` 90.0) (0.2 0.2 0.2)) "AdjustIfPossibleButAlwaysSpawn" "OverrideRootScale" (`self.GetOwner`) (`self.GetInstigator`))
  (return))

(fn `FireSwords`
  (bind _returnvalue (`self.GetOwner`))
  (bind _returnvalue_2 (`self.GetInstigator`))
  (bind _returnvalue_3 (`KismetMathLibrary.MakeRotator` 90.0))
  (bind _returnvalue_4 (+ (`SceneComponent.K2_GetComponentLocation` (`self.DefaultSceneRoot`)) (0.0 0.0 800.0)))
  (`|SpawnActorFromClass` "/Game/Blueprints/Damage/RainySword.RainySword_C" (`KismetMathLibrary.MakeTransform` _returnvalue_4 _returnvalue_3 (0.2 0.2 0.2)) "Undefined" "OverrideRootScale" _returnvalue _returnvalue_2)
  (`|SpawnActorFromClass` "/Game/Blueprints/Damage/RainySword.RainySword_C" (`KismetMathLibrary.MakeTransform` (+ _returnvalue_4 (300.0 0.0 0.0)) _returnvalue_3 (0.2 0.2 0.2)) "Undefined" "OverrideRootScale" _returnvalue _returnvalue_2)
  (`|SpawnActorFromClass` "/Game/Blueprints/Damage/RainySword.RainySword_C" (`KismetMathLibrary.MakeTransform` (- _returnvalue_4 (300.0 0.0 0.0)) _returnvalue_3 (0.2 0.2 0.2)) "Undefined" "OverrideRootScale" _returnvalue _returnvalue_2)
  (`|SpawnActorFromClass` "/Game/Blueprints/Damage/RainySword.RainySword_C" (`KismetMathLibrary.MakeTransform` (+ _returnvalue_4 (0.0 300.0 0.0)) _returnvalue_3 (0.2 0.2 0.2)) "Undefined" "OverrideRootScale" _returnvalue _returnvalue_2)
  (return))

(fn `UserConstructionScript`
  (`parent.UserConstructionScript`))