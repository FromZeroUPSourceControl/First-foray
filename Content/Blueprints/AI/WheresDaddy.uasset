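; Behavior tree decorator that checks whether the AI pawn has strayed beyond a leash distance from its "Daddy" actor.
; The condition check caches the owner's AI controller, then compares the straight-line distance between its pawn and the blackboard DaddyRef actor against DaddyLeash.
; It passes when that distance exceeds the leash, with no validity check on the Daddy actor.
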(fn `PerformConditionCheck`
  (params (OwnerActor :type "Actor Object Reference"))
  (returns (ReturnValue :type Boolean))
  (if (== (`self.AIControllerRef`) null)
    (set `self.AIControllerRef` (`AIBlueprintHelperLibrary.GetAIController` OwnerActor)))
  (return (> (`KismetMathLibrary.VSize` (- (`Actor.K2_GetActorLocation` (`BTFunctionLibrary.GetBlackboardValueAsActor` (`self.DaddyRef`))) (`Actor.K2_GetActorLocation` (`Controller.K2_GetPawn` (`self.AIControllerRef`))))) (`self.DaddyLeash`))))