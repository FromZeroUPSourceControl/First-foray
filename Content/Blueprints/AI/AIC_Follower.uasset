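; AIC_Follower is an AI controller for a follower character, driven by the BT_Follower behavior tree.
; On BeginPlay it stores the first player's pawn as DaddyActor through MakeDaddy and initializes BB_Follower.
; It then writes its own pawn's starting location to HomeLoc and the player pawn to DaddyRef before running the tree.
; All setup happens once, with no Tick logic or possession event.
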(event `self.ReceiveBeginPlay`
  (bind _returnvalue (`AIBlueprintHelperLibrary.GetBlackboard` self))
  (`self.MakeDaddy` (`self.K2_GetPawn` (`GameplayStatics.GetPlayerController` 0)))
  (`self.UseBlackboard` "/Game/Blueprints/AI/BB_Follower.BB_Follower")
  (`BlackboardComponent.SetValueAsVector` _returnvalue (`self.HomeLoc`) (`self.K2_GetActorLocation` (`self.K2_GetPawn` self)))
  (`BlackboardComponent.SetValueAsObject` _returnvalue (`self.DaddyRef`) (`self.DaddyActor`))
  (`self.RunBehaviorTree` "/Game/Blueprints/AI/BT_Follower.BT_Follower"))

(fn `MakeDaddy`
  (params (DaddyPawn :type "Pawn Object Reference"))
  (set `self.DaddyActor` DaddyPawn)
  (return))

(fn `UserConstructionScript`)