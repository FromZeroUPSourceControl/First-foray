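; Behavior tree task that sends an AIC_Follower's pawn toward the actor in the TargetToFollow blackboard key.
; It caches the controller on first execution, then issues AIMoveTo on the controlled pawn.
; The task finishes successfully as soon as the move is issued, without waiting for arrival.
; The move's success and failure callbacks also call FinishExecute.
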(event `self.ReceiveExecuteAI`
  (params (OwnerController :type "AIController Object Reference") (ControlledPawn :type "Pawn Object Reference"))
  (if (not (!= (`self.AIControllerRef`) null))
    (bind _asaic_follower (cast `/Game/Blueprints/AI/AIC_Follower` OwnerController))
    (set `self.AIControllerRef` _asaic_follower))
  (`|AIMoveTo` (`Controller.K2_GetPawn` (`self.AIControllerRef`)) (0.0 0.0 0.0) (`BTFunctionLibrary.GetBlackboardValueAsActor` (`self.TargetToFollow`))
    (:`then`
      (`self.FinishExecute` true :!label _label))
    (:`OnSuccess`
      (goto _label))
    (:`OnFail`
      (`self.FinishExecute` false))))