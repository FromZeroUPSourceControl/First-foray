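; DaddyTracker is a behavior tree service that tracks a "Daddy" actor for an AI by line of sight.
; Each tick it caches the owning controller if unset, then runs a visibility line trace from the controlled pawn to DaddyRef.
; When the trace hits that actor, it writes the actor and its location to the blackboard.
; It never clears these keys, so the last seen location persists after sight is lost.
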(event `self.ReceiveTickAI`
  (params (OwnerController :type "AIController Object Reference") (ControlledPawn :type "Pawn Object Reference") (DeltaSeconds :type "Float (single-precision)"))
  (bind _daddyref (`self.DaddyRef`))
  (bind _returnvalue (`Actor.K2_GetActorLocation` _daddyref))
  (if (not (!= (`self.AIControllerRef`) null))
    (set `self.AIControllerRef` OwnerController))
  (bind _output_get (set `self.SelfLoc` (`Actor.K2_GetActorLocation` ControlledPawn)))
  (bind _outhit (`KismetSystemLibrary.LineTraceSingle` _output_get _returnvalue "TraceTypeQuery1"))
  (if (== (`.HitActor` (`GameplayStatics.BreakHitResult` _outhit)) _daddyref)
    (`BTFunctionLibrary.SetBlackboardValueAsObject` (`self.ActorDaddy`) _daddyref)
    (`BTFunctionLibrary.SetBlackboardValueAsVector` (`self.DaddyLoc`) _returnvalue)))