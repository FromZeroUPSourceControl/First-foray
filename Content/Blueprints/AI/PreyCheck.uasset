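; PreyCheck is a behavior tree node that scans for targets its AI-controlled Humanoid reacts negatively to.
; On each AI tick it lazily caches the AIC_Follower controller and the pawn's Conscience component, then runs a multi-sphere object trace.
; Hit actors with a PNC_Concscience component have their mood passed to CheckReact.
; The first negative result writes that actor and its location to the blackboard as the move target.
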(event `self.ReceiveTickAI`
  (params (OwnerController :type "AIController Object Reference") (ControlledPawn :type "Pawn Object Reference") (DeltaSeconds :type "Float (single-precision)"))
  (if (not (!= (`self.AIControllerRef`) null))
    (bind _asaic_follower (cast `/Game/Blueprints/AI/AIC_Follower` OwnerController))
    (set `self.AIControllerRef` _asaic_follower))
  (if (not (!= (`self.ConscienceRef`) null))
    (bind _ashumanoid (cast `/Game/Blueprints/Archetypes/Humanoid` ControlledPawn))
    (set `self.ConscienceRef` (`/Game/Blueprints/Archetypes/Humanoid.ConscienceComponent` _ashumanoid)))
  (bind _outhits (`KismetSystemLibrary.SphereTraceMultiForObjects` (0.0 0.0 0.0) (0.0 0.0 0.0) 0.0 (`self.TarObjTypes`)))
  (for _array_element _outhits
    (bind (_bblockinghit _binitialoverlap _time _distance _location _impactpoint _normal _impactnormal _physmat _hitactor) (`GameplayStatics.BreakHitResult` _array_element))
    (bind _returnvalue (`Actor.GetComponentByClass` _hitactor "/Game/Blueprints/ActorComponents/PNC_Concscience.PNC_Concscience_C"))
    (if (`KismetSystemLibrary.IsValid` _returnvalue)
      (bind _judgement (`/Game/Blueprints/ActorComponents/PNC_Concscience.CheckReact` (`self.ConscienceRef`) (`/Game/Blueprints/ActorComponents/PNC_Concscience.GetMood` _returnvalue)))
      (if (< _judgement 0)
        (`BTFunctionLibrary.SetBlackboardValueAsObject` (`self.MoveToTar`) _hitactor)
        (`BTFunctionLibrary.SetBlackboardValueAsVector` (`self.TargetLoc`) _location)
        (break)))))