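; Behavior Tree decorator that checks whether an AI pawn is within its personal space bubble around its move target.
; PerformConditionCheck gets the AI controller from the owner actor and reads the target actor from the MoveToTar blackboard key.
; It passes when the distance between the controlled pawn and that target is at most BubbleRadius.
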(fn `PerformConditionCheck`
  (params (OwnerActor :type "Actor Object Reference"))
  (returns (ReturnValue :type Boolean))
  (bind _returnvalue (`AIBlueprintHelperLibrary.GetAIController` OwnerActor))
  (if (== _returnvalue null)
    (set `self.AIControllerRef` _returnvalue)
    (return (<= (`KismetMathLibrary.VSize` (- (`Actor.K2_GetActorLocation` (`BTFunctionLibrary.GetBlackboardValueAsActor` (`self.MoveToTar`))) (`Actor.K2_GetActorLocation` (`Controller.K2_GetPawn` (`self.AIControllerRef`))))) (`self.BubbleRadius`)))))