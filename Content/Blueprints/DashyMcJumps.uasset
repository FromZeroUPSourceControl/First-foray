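; DashyMcJumps is a player input Blueprint that handles temporary class switching and manual camera control.
; SwitchClass increments an index into a pawn array and possesses that pawn, except on wrap-around, where it only resets the index to zero.
; Mouse axes accumulate scaled yaw and pitch into a shared control rotation update, ignoring pitch input that would go beyond straight up or down.
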(event `InputAction|SwitchClass`
  (params (Key :type "Key Structure" :default "AnyKey"))
  ;[1 0.3018 0.3217] Temp class switch function
  (:`Pressed`
    (bind _result (`/Engine/EditorBlueprintResources/StandardMacros.IncrementInt` (`self.CharaSelect`))
      (:`  `
        (if (== (mod _result (`KismetArrayLibrary.Array_Length` (`self.PawnArraySwitchClass`))) 0)
          (set `self.CharaSelect` 0)
          (else
            ;[1 0.2462 0] Class Switch (archetype swap)
            (`self.Possess` (`GameplayStatics.GetPlayerController` (`self.PlayerControllerIndex`)) (`|GetArrayItem` (`self.PawnArraySwitchClass`) (`self.CharaSelect`)))))))))

(event `InputAxis|MouseLeftRight` :overrideparent false
  (params (AxisValue :type "Float (single-precision)"))
  ;[1 0.2462 0] Super Camera Control
  (bind _output_get (set `self.ControllerYaw` (+ (`self.ControllerYaw`) (* (`self.InputYawScale`) AxisValue))))
  (`self.SetControlRotation` (`KismetMathLibrary.MakeRotator` 0.0 (stale `InputAxis|MouseUpDown` _output_get) _output_get) :!label _label))

(event `InputAxis|MouseUpDown` :overrideparent false
  (params (AxisValue :type "Float (single-precision)"))
  (bind _returnvalue (+ (* AxisValue (`self.InputPitchScale`)) (`self.ControllerPitch`)))
  ;[1 0.2462 0] Super Camera Control
  (if (and (<= _returnvalue 90.0) (>= _returnvalue -90.0))
    (bind _output_get (set `self.ControllerPitch` _returnvalue))
    (goto _label)))

(fn `UserConstructionScript`)