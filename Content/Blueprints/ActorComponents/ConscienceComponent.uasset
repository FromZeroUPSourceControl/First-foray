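; ConscienceComponent is an actor component that holds faction attitudes and scores an impression against them.
; CheckReact walks the impression's entries, decrementing a counter and folding each matching attitude into a clamped judgement weighted by that countdown.
; The walk stops at the first entry without an attitude or when the counter runs out.
; Accessors get and set the attitude map, GetMood returns stored associations, and the event graph is empty.
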(event `self.ReceiveBeginPlay`)

(fn `CheckReact`
  (params (Impression :type "Array of /Game/Blueprints/Data/Enumerations/E_Factions Enum" :default _))
  (returns (Judgement :type Integer))
  (locals (AssocLoc :type "Array of /Game/Blueprints/Data/Enumerations/E_Factions Enum") (Judgenation :type Integer) (BeanCounterDown :type Integer :default 3))
  (bind _beancounterdown (`local.BeanCounterDown`))
  (bind _output_get (set `local.AssocLoc` Impression))
  (for _array_element _output_get
    (bind (_value _returnvalue) (`BlueprintMapLibrary.Map_Find` (`self.FactionAttitudes`) _array_element))
    (if (and _returnvalue (> (`local.BeanCounterDown`) 0))
      (`/Engine/EditorBlueprintResources/StandardMacros.DecrementInt` _beancounterdown
        (:`  `
          (bind _output_get_2 (set `local.Judgenation` (`KismetMathLibrary.Clamp` (+ _value (* _beancounterdown (`local.Judgenation`))) 0 1000)))))
      (else
        (break))))
  (return _output_get_2))

(fn `GetAttitudes`
  (returns (FactionAttitudes :type "Map of /Game/Blueprints/Data/Enumerations/E_Factions Enum to Integer"))
  (return (`self.FactionAttitudes`)))

(fn `GetMood`
  (returns (Associations :type "Array of /Game/Blueprints/Data/Enumerations/E_Factions Enum"))
  (return (`self.Associations`)))

(fn `SetAttitudes`
  (params (Attitudes :type "Map of /Game/Blueprints/Data/Enumerations/E_Factions Enum to Integer" :default _))
  (set `self.FactionAttitudes` Attitudes))