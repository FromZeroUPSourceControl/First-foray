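; Actor component on the PlayerVessel that stores the player's skills and handles activating and upgrading them.
; ActivateSkill maps a slot to stored skill data, checks learned, active and cooldown state, then dispatches Sword Rain or Slash Dash.
; Sword Rain traces from the camera to place a stage-scaled targeting actor; Slash Dash runs on the owner.
; IncrSkillStage spends upgrade points, raising stage and doubling cost; Sword Aura and FireSkill are empty stubs.
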(event `self.ReceiveBeginPlay`
  (bind _asplayer_vessel (cast `/Game/Blueprints/Archetypes/PlayerVessel` (`self.GetOwner`))
    (:`then`
      (set `self.PV_Owner` _asplayer_vessel))
    (:`CastFailed`
      (`KismetSystemLibrary.PrintText` "Master skill handler get character cast failed!"))))

(fn `ActivateSkill`
  (params (Slot :type Integer))
  (locals (E_SkillType :type "/Game/Blueprints/Data/Enumerations/E_Skills Enum"))
  (bind _pv_owner (`self.PV_Owner`))
  (bind _output (`|GetArrayItem` (`self.SkillSlots`) Slot))
  (bind (_value _returnvalue) (`BlueprintMapLibrary.Map_Find` (`self.SkillsStor`) _output))
  (bind ((`IsActive_32_F69589E0441231822E677F9CEB83527B` _isactive) (`SkillStage_21_300FEE3943C7564926E6C19B13E1EB5F` _skillstage)) (break `/Game/Blueprints/Data/DataStructures/S_SkillData` _value))
  (if _returnvalue
    (bind _output_get (set `local.E_SkillType` _output))
    (if (> _skillstage 0)
      (if _isactive
        (if (> (`BlueprintMapLibrary.Map_Find` (`/Game/Blueprints/Archetypes/PlayerVessel.Cooldowns` _pv_owner) _output_get) 0.0)
          (`KismetSystemLibrary.PrintText` "Skill is on cooldown.")
          (else
            (switch `/Game/Blueprints/Data/Enumerations/E_Skills` _output_get
              (:`NewEnumerator0`
                _)
              (:`NewEnumerator1`
                (if (`/Game/Blueprints/Archetypes/PlayerVessel.Targeting` _pv_owner)
                  (`KismetSystemLibrary.PrintText` "One target at a time, please.")
                  (else
                    (`self.Cast_SwordRain`)
                    (return))))
              (:`NewEnumerator2`
                (`self.Cast_SlashDash`)
                (return)))))
        (else
          (`KismetSystemLibrary.PrintText` "Skill is not ready." true true (struct :`R` 1.0 :`G` 0.305122 :`B` 0.455616 :`A` 1.0))))
      (else
        (`KismetSystemLibrary.PrintText` "Skill has not been learned.")))
    (else
      (`KismetSystemLibrary.PrintText` "Index Out of Bounds - Skill Activation" true true (struct :`G` 0.66 :`B` 1.0 :`A` 1.0) 10.0)))
  (return))

(fn `Cast_SlashDash`
  (bind _cooldowns (`/Game/Blueprints/Archetypes/PlayerVessel.Cooldowns` (`self.PV_Owner`)))
  (if (<= (`BlueprintMapLibrary.Map_Find` _cooldowns "NewEnumerator2") 0.0)
    (`/Game/Blueprints/Archetypes/PlayerVessel.SlashDashExecute` (`self.PV_Owner`) (`self.SlashDashTargets`) (`self.SlashDashDamage`))
    (`BlueprintMapLibrary.Map_Add` _cooldowns "NewEnumerator2" (`.Cooldown_42_472C2A7843D18ACC414C849552952460` (break `/Game/Blueprints/Data/DataStructures/S_SkillData` (`BlueprintMapLibrary.Map_Find` (`self.SkillsStor`) "NewEnumerator2"))))
    (return)
    (else
      (`KismetSystemLibrary.PrintText` "Cooldown!")
      (return))))

(fn `Cast_SwordAura`)

(fn `Cast_SwordRain`
  (locals (SwordRainTerrainCastObjectTypes :type "Array of EObjectTypeQuery Enum"))
  (bind _pv_owner (`self.PV_Owner`))
  (bind _playercam (`/Game/Blueprints/Archetypes/PlayerVessel.PlayerCam` (`self.PV_Owner`)))
  (bind ((`SkillStage_21_300FEE3943C7564926E6C19B13E1EB5F` _skillstage) (`Cooldown_42_472C2A7843D18ACC414C849552952460` _cooldown)) (break `/Game/Blueprints/Data/DataStructures/S_SkillData` (`BlueprintMapLibrary.Map_Find` (`self.SkillsStor`) "NewEnumerator1")))
  (bind _returnvalue (`SceneComponent.K2_GetComponentLocation` _playercam))
  (bind _returnvalue_2 (`KismetMathLibrary.GreaterGreater_VectorRotator` (+ _returnvalue (* (`SceneComponent.GetForwardVector` _playercam) 1500.0)) (`SceneComponent.K2_GetComponentRotation` _playercam)))
  (bind (_outhit _returnvalue_3) (`KismetSystemLibrary.LineTraceSingleForObjects` _returnvalue _returnvalue_2 (`local.SwordRainTerrainCastObjectTypes`)))
  (if _returnvalue_3
    (set `self.SwordRainPN_SpawnTransform` (`KismetMathLibrary.MakeTransform` (`.Location` (`GameplayStatics.BreakHitResult` _outhit)) (struct) (0.5 0.5 1.0)))
    (else
      (set `self.SwordRainPN_SpawnTransform` (`KismetMathLibrary.MakeTransform` _returnvalue_2 (struct) (0.5 0.5 1.0)))))
  (bind _returnvalue_4 (`|SpawnActorFromClass` "/Game/Blueprints/PropNinjas/PN_S_SwordRain.PN_S_SwordRain_C" (`self.SwordRainPN_SpawnTransform`) "Undefined" "OverrideRootScale" _pv_owner (* _skillstage 5) _pv_owner _pv_owner))
  (`/Game/Blueprints/Archetypes/PlayerVessel.SetTarget` _pv_owner _returnvalue_4 "NewEnumerator1")
  (`BlueprintMapLibrary.Map_Add` (`/Game/Blueprints/Archetypes/PlayerVessel.Cooldowns` _pv_owner) "NewEnumerator1" _cooldown)
  (return))

(fn `FireSkill`)

(fn `IncrSkillStage`
  (params (SkillSelection :type "/Game/Blueprints/Data/Enumerations/E_Skills Enum" :default "NewEnumerator0"))
  (locals (SkillSelect :type "/Game/Blueprints/Data/Enumerations/E_Skills Enum"))
  (bind _skillsstor (`self.SkillsStor`))
  (bind (_value _returnvalue) (`BlueprintMapLibrary.Map_Find` _skillsstor (`local.SkillSelect`)))
  (bind (_skilldisplayname _skilldescription _isactive _skillname _skillstage _skillicon _skillpointcost _cooldown) (break `/Game/Blueprints/Data/DataStructures/S_SkillData` _value))
  (set `local.SkillSelect` SkillSelection)
  (if _returnvalue
    (bind _valid (`/Game/Blueprints/Archetypes/PlayerVessel.ModifyUpgradePoints` (`self.PV_Owner`) 1 (- 0 _skillpointcost)))
    (if _valid
      (`BlueprintMapLibrary.Map_Add` _skillsstor (`local.SkillSelect`) (make `/Game/Blueprints/Data/DataStructures/S_SkillData` _skilldisplayname _skilldescription true _skillname (+ _skillstage 1) _skillicon (* _skillpointcost 2) _cooldown))
      (return)
      (else
        (return)))
    (else
      (return))))