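; RainySword is a sword projectile that deals heavy Physical damage, credited to its instigator's controller and pawn.
; On BeginPlay, the MoveSeg1 timeline drives local Z velocity while incrementally rolling the actor.
; When that finishes, MoveSegAtt drives the attack mostly along local Y, with a slight Z component.
; Any Box overlap applies damage and destroys the actor, without filtering what it hits.
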(event `self.ReceiveBeginPlay`
  (bind _projectilemovement (`self.ProjectileMovement`))
  (`ProjectileMovementComponent.SetVelocityInLocalSpace` _projectilemovement (0.0 0.0 400.0))
  (bind (_direction _rotation _velocity) (`Timeline|MoveSeg1`)
    (:`Update`
      (`ProjectileMovementComponent.SetVelocityInLocalSpace` _projectilemovement (`KismetMathLibrary.MakeVector` 0.0 0.0 _velocity))
      (`self.K2_AddActorLocalRotation` (`KismetMathLibrary.MakeRotator` _rotation)))
    (:`Finished`
      (bind (_direction_2 _velocity_2) (`Timeline|MoveSegAtt`)
        (:`Update`
          (`ProjectileMovementComponent.SetVelocityInLocalSpace` (`self.ProjectileMovement`) (`KismetMathLibrary.MakeVector` 0.0 _velocity_2 (/ _velocity_2 50.0))))))))

(event `self.Box.OnComponentBeginOverlap`
  (params (OverlappedComponent :type "PrimitiveComponent Object Reference") (OtherActor :type "Actor Object Reference") (OtherComp :type "PrimitiveComponent Object Reference") (OtherBodyIndex :type Integer) (bFromSweep :type Boolean) (SweepResult :type "HitResult Structure (by ref)"))
  (bind _returnvalue (`self.GetInstigatorController`))
  (`GameplayStatics.ApplyDamage` OtherActor 200.0 _returnvalue (`Controller.K2_GetPawn` _returnvalue) "/Game/Blueprints/Damage/DamageTypes/Physical.Physical_C")
  (`self.K2_DestroyActor`))

(fn `UserConstructionScript`
  (`parent.UserConstructionScript`))